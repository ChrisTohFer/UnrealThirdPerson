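; Player character Blueprint handling aiming, shooting zombies, picking up items and toggling doors.
; Aim plays a timeline that drives camera boom arm length and sets an aim flag, reversing and clearing them on release.
; Fire plays a gunshot and line-traces from the gun along camera forward, reducing a hit Zombie's health.
; PickUpItem uses short traces from the same origin to pick up BaseItems or toggle Doors.
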(event `InputAction|Aim`
  (params (Key :type "Key Structure"))
  ;[1 1 1] Aim Camera
  (:`Pressed`
    (bind (_direction _curve) (`Timeline|CameraAimCurve` :!label _label)
      (:`Update`
        (set `SpringArmComponent.TargetArmLength` _curve (`self.CameraBoom`)))))
  (:`Released`
    (goto _label :!via `Reverse`)))

(event `InputAction|Aim`
  (params (Key :type "Key Structure"))
  ;[1 1 1] Aim Animation
  (:`Pressed`
    (set `self.Aim Button Down` true))
  (:`Released`
    (set `self.Aim Button Down` false)))

(event `InputAction|Fire`
  (params (Key :type "Key Structure"))
  (bind _returnvalue (+ (`self.K2_GetActorLocation` (`self.Gun`)) (-2.5 8.0 11.0)))
  ;[1 1 1] Fire Gun
  (:`Pressed`
    (`GameplayStatics.SpawnSoundAtLocation` "/Game/Audio/Smg/SMGFire_2.SMGFire_2" (`self.K2_GetActorLocation` (`self.Gun`)) (struct) 0.2 1.0 0.0 null null)
    (bind _outhit (`KismetSystemLibrary.LineTraceSingle` :`Start` _returnvalue :`End` (+ _returnvalue (* (`KismetMathLibrary.GetForwardVector` (`self.K2_GetActorRotation` (`GameplayStatics.GetPlayerCameraManager` 0))) 1500.0)) :`TraceChannel` "TraceTypeQuery1" :`DrawDebugType` "ForOneFrame"))
    (bind _aszombie (cast `/Game/Blueprints/Zombie` (`.HitActor` (`GameplayStatics.BreakHitResult` _outhit))))
    (bind _output_get (set `/Game/Blueprints/Zombie.Health` (- (stale _output_get) 1.0) _aszombie))))

(event `InputAction|PickUpItem`
  (params (Key :type "Key Structure"))
  (bind _returnvalue (+ (`self.K2_GetActorLocation` (`self.Gun`)) (-2.5 8.0 11.0)))
  ;[1 1 1] Item Pickup
  (:`Pressed`
    (bind _outhit (`KismetSystemLibrary.LineTraceSingle` :`Start` _returnvalue :`End` (+ _returnvalue (* (`KismetMathLibrary.GetForwardVector` (`self.K2_GetActorRotation` (`GameplayStatics.GetPlayerCameraManager` 0))) 100.0)) :`TraceChannel` "TraceTypeQuery1" :`DrawDebugType` "ForOneFrame"))
    (bind _asbase_item (cast `BaseItem` (`.HitActor` (`GameplayStatics.BreakHitResult` _outhit))))
    (`BaseItem.PickUpItem` _asbase_item)))

(event `InputAction|PickUpItem`
  (params (Key :type "Key Structure"))
  (bind _returnvalue (+ (`self.K2_GetActorLocation` (`self.Gun`)) (-2.5 8.0 11.0)))
  ;[1 1 1] Door Open
  (:`Pressed`
    (bind _outhit (`KismetSystemLibrary.LineTraceSingle` :`Start` _returnvalue :`End` (+ _returnvalue (* (`KismetMathLibrary.GetForwardVector` (`self.K2_GetActorRotation` (`GameplayStatics.GetPlayerCameraManager` 0))) 100.0)) :`TraceChannel` "TraceTypeQuery1" :`DrawDebugType` "ForOneFrame"))
    (bind _asdoor (cast `/Game/Blueprints/Door` (`.HitActor` (`GameplayStatics.BreakHitResult` _outhit))))
    (if (== (`/Game/Blueprints/Door.Opened` _asdoor) false)
      (set `/Game/Blueprints/Door.Opened` true _asdoor)
      (else
        (set `/Game/Blueprints/Door.Opened` false _asdoor)))
    (`/Game/Blueprints/Door.ToggleDoor` _asdoor)))

(fn `UserConstructionScript`
  (`parent.UserConstructionScript`))