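; Trigger volume actor that plays a level sequence cutscene when the player walks into it, with an optional zombie spawn afterwards.
; Overlap by a PlayerObject starts the referenced sequence and switches the trigger to NoCollision so it fires only once.
; When SpawnZombie is set, a delay using the sequence's playback end value precedes spawning a Zombie at the SpawnTransform actor's transform.
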(event `self.Trigger.OnComponentBeginOverlap`
  (params (OverlappedComponent :type "PrimitiveComponent Object Reference") (OtherActor :type "Actor Object Reference") (OtherComp :type "PrimitiveComponent Object Reference") (OtherBodyIndex :type Integer) (bFromSweep :type Boolean) (SweepResult :type "HitResult Structure (by ref)"))
  (bind _sequenceplayer (`LevelSequenceActor.SequencePlayer` (`self.Sequence`)))
  (cast `/Game/Blueprints/PlayerObject` OtherActor)
  (`MovieSceneSequencePlayer.Play` _sequenceplayer)
  (`PrimitiveComponent.SetCollisionProfileName` (`self.Trigger`) "NoCollision")
  (if (`self.SpawnZombie`)
    (`KismetSystemLibrary.Delay` (`MovieSceneSequencePlayer.GetPlaybackEnd` _sequenceplayer))
    (`|SpawnActorFromClass` "/Game/Blueprints/Zombie.Zombie_C" (`self.GetTransform` (`self.SpawnTransform`)) "Undefined" "OverrideRootScale" null null)))

(fn `UserConstructionScript`)