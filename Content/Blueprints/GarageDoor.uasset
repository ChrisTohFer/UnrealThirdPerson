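; GarageDoor is a Blueprint for a door that opens when a named key item is present in the inventory.
; ToggleCardReader looks up KeyName in the inventory and, if the item exists and the door is still closed, instantly moves the Door component's owning actor upward by a fixed offset.
; An Opened flag makes this one-way, with no closing logic or animation despite the toggle name.
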(fn `ToggleCardReader`
  (bind _returnvalue (`BaseInventory.GetInventory`))
  (bind _returnvalue_2 (`BaseInventory.GetItemByName` _returnvalue (`self.KeyName`)))
  (`/Engine/EditorBlueprintResources/StandardMacros.IsValid` _returnvalue_2
    (:`Is Valid`
      (if (== (`self.Opened`) false)
        (`self.K2_SetActorLocation` (`ActorComponent.GetOwner` (`self.Door`)) (`KismetMathLibrary.MakeVector` (.x (`SceneComponent.K2_GetComponentLocation` (`self.Door`))) (.y (`SceneComponent.K2_GetComponentLocation` (`self.Door`))) (+ (.z (`SceneComponent.K2_GetComponentLocation` (`self.Door`))) 250.0)) false false)
        (set `self.Opened` true)))))

(fn `UserConstructionScript`)